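; Player controller for placing cubes on a 100-unit grid with the mouse, with the cursor shown from BeginPlay.
; Holding key 1, 2 or 3 selects a cube type, and releasing it resets the type to the value that blocks placement.
; A left click traces under the cursor, snaps the hit to a cell center at fixed height, then spawns BP_Cube and starts its mesh setup and animation.
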(event EventBeginPlay
  (Variables|Default|SetbShowMouseCursor true))

(event Input|KeyboardEvents|3
  (params (Key :type Key%20Structure :default "None"))
  (:Pressed
    (Variables|Default|SetCurCubeType "NewEnumerator2"))
  (:Released
    (Variables|Default|SetCurCubeType "NewEnumerator3")))

(event Input|KeyboardEvents|1
  (params (Key :type Key%20Structure :default "None"))
  (:Pressed
    (Variables|Default|SetCurCubeType "NewEnumerator0"))
  (:Released
    (Variables|Default|SetCurCubeType "NewEnumerator3")))

(event Input|KeyboardEvents|2
  (params (Key :type Key%20Structure :default "None"))
  (:Pressed
    (Variables|Default|SetCurCubeType "NewEnumerator1"))
  (:Released
    (Variables|Default|SetCurCubeType "NewEnumerator3")))

(event Input|MouseEvents|LeftMouseButton
  (params (Key :type Key%20Structure :default "None"))
  (bind (_hitresult _returnvalue) (Game|Player|GetHitResultUnderCursorbyChannel "TraceTypeQuery1" true))
  (bind _location (Collision|BreakHitResult _hitresult))
  (bind (_x _y) (Math|Vector|BreakVector _location))
  (:Pressed
    (if (not (Utilities|Enum|Equal(Enum) (Variables|Default|GetCurCubeType) "NewEnumerator3"))
      (if _returnvalue
        (bind _returnvalue_2 (Game|SpawnActorfromClass "/Game/Cube/BP_Cube.BP_Cube_C" (Math|Transform|MakeTransform (Math|Vector|MakeVector (CallFunction|Normalize _x) (CallFunction|Normalize _y) 7e+01)) "Undefined" 0 0))
        (Default|InitMeshandStartAnim _returnvalue_2 (Variables|Default|GetCurCubeType))))))

(fn ConstructionScript)

(fn Normalize
  (params (Input :type Float%20%28single-precision%29))
  (return (+ (* (/ (Math|Float|Truncate Input) 100) 1e+02) (select (>= Input 0.0) 5e+01 -5e+01))))